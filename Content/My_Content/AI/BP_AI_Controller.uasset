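; AI controller for BP_AI_Char that starts its behavior tree on possession and feeds perception results into the blackboard.
; It always runs the passive tree, because the aggressive branch is hard-wired off and the random aggression flag is unused.
; Sight sets or clears the seen target, while hearing sets or clears the last heard location and prints it.
; A damage-sense check that updates the alive key from health is disconnected.
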(event `self.ReceivePossess`
  (params (PossessedPawn :type "Pawn Object Reference"))
  (bind _asbp_ai_char (cast `/Game/My_Content/AI/BP_AI_Char` PossessedPawn))
  (set `self.Possessed Pawn` _asbp_ai_char)
  (set `self.Is_Agressive_Bot?` (`KismetMathLibrary.RandomBool`))
  (if false
    (bind _returnvalue (`self.RunBehaviorTree` "/Game/My_Content/AI/Agressive_Behavior/BT_Agressive_AI_Char.BT_Agressive_AI_Char"))
    (if _returnvalue
      (`self.UseBlackboard` "/Game/My_Content/AI/Agressive_Behavior/BB_Agressive_AI_Char.BB_Agressive_AI_Char"))
    (else
      (bind _returnvalue_2 (`self.RunBehaviorTree` "/Game/My_Content/AI/Passive_Behavior/BT_Passive_AI_Char.BT_Passive_AI_Char"))
      (if _returnvalue_2
        (`self.UseBlackboard` "/Game/My_Content/AI/Passive_Behavior/BB_Passive_AI_Char.BB_Passive_AI_Char")))))

(event `self.AIPerception.OnTargetPerceptionInfoUpdated`
  (params (UpdateInfo :type "ActorPerceptionUpdateInfo Structure (by ref)"))
  (bind (_age _expirationage _strength _stimuluslocation _receiverlocation _tag _bsuccessfullysensed) (break `AIStimulus` UpdateInfo_Stimulus))
  (bind _returnvalue (`AIBlueprintHelperLibrary.GetBlackboard` null))
  (bind _returnvalue_2 (`KismetStringLibrary.Conv_StringToName` "LastLocHeardSomething"))
  (bind _returnvalue_3 (`BlackboardComponent.GetValueAsVector` _returnvalue _returnvalue_2))
  (bind _returnvalue_4 (`AIPerceptionSystem.GetSenseClassForStimulus` UpdateInfo_Stimulus))
  (if (== _returnvalue_4 "/Script/AIModule.AISense_Sight")
    (if _bsuccessfullysensed
      (`BlackboardComponent.SetValueAsObject` (`AIBlueprintHelperLibrary.GetBlackboard` null) (`KismetStringLibrary.Conv_StringToName` "PlayerRef") UpdateInfo_Target)
      (`BlackboardComponent.SetValueAsBool` (`AIBlueprintHelperLibrary.GetBlackboard` null) (`KismetStringLibrary.Conv_StringToName` "SeePlayerNow?") true)
      (else
        (`BlackboardComponent.ClearValue` (`AIBlueprintHelperLibrary.GetBlackboard` null) (`KismetStringLibrary.Conv_StringToName` "PlayerRef"))
        (`BlackboardComponent.SetValueAsBool` (`AIBlueprintHelperLibrary.GetBlackboard` null) (`KismetStringLibrary.Conv_StringToName` "SeePlayerNow?") false)))
    (else
      (bind _returnvalue_5 (`AIPerceptionSystem.GetSenseClassForStimulus` UpdateInfo_Stimulus))
      (if (== _returnvalue_5 "/Script/AIModule.AISense_Hearing")
        (if _bsuccessfullysensed
          (`BlackboardComponent.SetValueAsVector` _returnvalue _returnvalue_2 _stimuluslocation)
          (`KismetSystemLibrary.PrintString` (`KismetStringLibrary.Conv_VectorToString` _returnvalue_3))
          (else
            (`BlackboardComponent.ClearValue` _returnvalue _returnvalue_2)
            (`KismetSystemLibrary.PrintString` (`KismetStringLibrary.Conv_VectorToString` _returnvalue_3))))))))

(fn `UserConstructionScript`)