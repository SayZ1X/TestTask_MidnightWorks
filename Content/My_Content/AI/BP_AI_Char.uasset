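; BP_AI_Char is an AI character that fights with a pistol and has slide and climb movement.
; On BeginPlay it spawns a pistol at the right-hand socket and equips it; Fire falls back to reloading when the magazine is empty.
; Damage feeds a health component.
; A timeline resizes the capsule and moves the mesh for sliding, with a timed cooldown, while a forward sphere trace sets climb state and wall normal.
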(event `self.ReceiveBeginPlay`
  (bind _returnvalue (`|SpawnActorFromClass` "/Game/My_Content/Weapons/Firearm/BP_Pistol_For_AI.BP_Pistol_For_AI_C" (`SceneComponent.GetSocketTransform` (`self.Mesh`) "Right_hand" "RTS_World") "Undefined" "MultiplyWithRoot" self null))
  (`/Game/My_Content/Weapons/BPI_Pickup_For_AI.PickUp` _returnvalue self)
  (set `/Game/My_Content/Weapons/BP_Base_Weapon_For_AI.Is_Equipped?` true _returnvalue))

(event `self.ReceiveTick`
  (params (DeltaSeconds :type "Float (single-precision)")))

(event `Start_Change_Slide_Capsule_Size`
  (bind _capsulecomponent (`self.CapsuleComponent`))
  (bind (_returnvalue_x _returnvalue_y _returnvalue_z) (`KismetMathLibrary.BreakVector` (`SceneComponent.K2_GetComponentLocation` _capsulecomponent)))
  ;[1 1 1] Setup Sliding Capsule Size
  (bind (_direction _capsule_size) (`Timeline|Slide_Capsule_Size` :!label _label)
    (:`Update`
      (`CapsuleComponent.SetCapsuleHalfHeight` _capsulecomponent _capsule_size true)
      (`SceneComponent.K2_SetWorldLocation` (`self.Mesh`) (`KismetMathLibrary.MakeVector` _returnvalue_x _returnvalue_y (- _returnvalue_z (`CapsuleComponent.CapsuleHalfHeight` _capsulecomponent))) false false))))

(event `Slide_Was_Finished`
  ;[1 1 1] Make Slide Limit
  (set `self.Is_Sliding?` false)
  (set `self.Can_Sliding?` false)
  (`KismetSystemLibrary.K2_SetTimerDelegate` (delegate `Change_Slide_State`) (`self.Time_Between_Slides_ms`)))

(event `Reverse_Change_Slide_Capsule_Size`
  ;[1 1 1] Setup Sliding Capsule Size
  (goto _label :!via `Reverse`))

(event `Change_Slide_State`
  ;[1 1 1] Make Slide Limit
  (set `self.Can_Sliding?` true))

(event `Fire`
  (bind _equiped_weapon (`self.Equiped_Weapon`))
  (bind _can_fire_ (`/Game/My_Content/Weapons/BP_Base_Weapon_For_AI.Check_Can_Fire` _equiped_weapon))
  (if _can_fire_
    (`/Game/My_Content/Weapons/BP_Base_Weapon_For_AI.Fire` _equiped_weapon)
    (elif (<= (`/Game/My_Content/Weapons/BP_Base_Weapon_For_AI.Magazine_Capacity` _equiped_weapon) 0)
      (`self.Reload`))))

(event `Reload`
  (bind _equiped_weapon (`self.Equiped_Weapon`))
  (bind _can_reload_ (`/Game/My_Content/Weapons/BP_Base_Weapon_For_AI.Check_Can_Reload` _equiped_weapon))
  (if _can_reload_
    (`/Game/My_Content/Weapons/BP_Base_Weapon_For_AI.Reload` _equiped_weapon)))

(event `self.ReceiveAnyDamage`
  (params (Damage :type "Float (single-precision)") (DamageType :type "DamageType Object Reference") (InstigatedBy :type "Controller Object Reference") (DamageCauser :type "Actor Object Reference"))
  (`/Game/My_Content/Player_Character/BPC_Health_Component.Decrease Health` (`self.BPC_Health_Component`) Damage))

(fn `GetForwardVector`
  (returns (X :type "Float (double-precision)") (Y :type "Float (double-precision)") (Z :type "Float (double-precision)") (Rotation :type "Rotator Structure"))
  (bind (_returnvalue_x _returnvalue_y _returnvalue_z) (`KismetMathLibrary.BreakVector` (`self.K2_GetActorLocation`)))
  (bind (_returnvalue_x_2 _returnvalue_y_2) (`KismetMathLibrary.BreakVector` (+ (`self.K2_GetActorLocation`) (* (`self.GetActorForwardVector`) 50.0))))
  (return _returnvalue_x_2 _returnvalue_y_2 (+ _returnvalue_z 154.0) (`self.K2_GetActorRotation`)))

(fn `StartClimbing`
  (returns (Return_Value :type Boolean) (Climbing_Z_Yaw :type "Float (double-precision)"))
  (bind _returnvalue (+ (`self.K2_GetActorLocation`) (0.0 0.0 20.0)))
  ;[1 1 1] Trace sphere from head to forward
  (bind (_outhit _returnvalue_2) (`KismetSystemLibrary.SphereTraceSingle` :`Start` _returnvalue :`End` (+ _returnvalue (* (`self.GetActorForwardVector`) 44.0)) :`Radius` 6.0 :`TraceChannel` "TraceTypeQuery1" :`DrawDebugType` "ForDuration"))
  (if _returnvalue_2
    (set `self.Climb_Normal` (`.Normal` (`GameplayStatics.BreakHitResult` _outhit)))
    (set `self.Is_Climbing?` true)
    (else
      (set `self.Is_Climbing?` false)))
  (bind (_returnvalue_roll _returnvalue_pitch _returnvalue_yaw) (`KismetMathLibrary.BreakRotator` (`KismetMathLibrary.MakeRotFromX` (`.Normal` (`GameplayStatics.BreakHitResult` _outhit)))))
  (return _returnvalue_2 (+ _returnvalue_yaw 180.0)))

(fn `StopClimbing`
  (set `self.Is_Climbing?` false)
  (set `self.Mesh_Offset_When_Climb_Z` 70.0)
  (`CharacterMovementComponent.SetMovementMode` (`self.CharacterMovement`) "MOVE_Falling" 0)
  (set `self.Climb_Up_Down` 0.0)
  (set `self.Climb_Left_Right` 0.0))

(fn `UserConstructionScript`)