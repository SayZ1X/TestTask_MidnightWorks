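; Actor component that tracks health for player-project actors such as AI characters and barrels.
; It starts at max health on BeginPlay, subtracts incoming damage through DecreaseHealth, and calls DIE at zero or below.
; DIE casts the owner: AI characters ragdoll by enabling mesh physics and swapping collision profiles, while barrels only play an explosion sound.
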(event `self.ReceiveBeginPlay`
  (set `self.Current_Health` (`self.Max_Health`)))

(event `Decrease Health`
  (params (Taken_Damage :type "Float (double-precision)"))
  (bind _output_get (set `self.Current_Health` (- (`self.Current_Health`) Taken_Damage)))
  (if (<= _output_get 0.0)
    (`self.DIE`)))

(event `DIE`
  (bind _returnvalue (`self.GetOwner`))
  (bind _asbp_ai_char (cast `/Game/My_Content/AI/BP_AI_Char` _returnvalue)
    (:`then`
      (bind _mesh (`Character.Mesh` _asbp_ai_char))
      (`PrimitiveComponent.SetSimulatePhysics` _mesh true)
      (`PrimitiveComponent.SetCollisionProfileName` (`Character.CapsuleComponent` _asbp_ai_char) "NoCollision" true)
      (`PrimitiveComponent.SetCollisionProfileName` _mesh "Ragdoll" true))
    (:`CastFailed`
      (bind _asbp_barrel (cast `/Game/My_Content/Blueprints/BP_Barrel` _returnvalue))
      (`GameplayStatics.PlaySound2D` "/Game/StarterContent/Audio/Explosion01.Explosion01" 1.0 1.0 0.0 null _asbp_barrel))))