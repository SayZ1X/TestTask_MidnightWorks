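; BP_Barrel is a destructible barrel that explodes once damage depletes its health.
; AnyDamage feeds a health component; at zero it spawns a particle effect and deals full radial damage equal to the last hit, ignoring itself.
; The mesh is launched upward with a random horizontal impulse, then the actor is destroyed after a short delay.
; No guard stops further hits during that delay from repeating the explosion.
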(event `self.ReceiveAnyDamage`
  (params (Damage :type "Float (single-precision)") (DamageType :type "DamageType Object Reference") (InstigatedBy :type "Controller Object Reference") (DamageCauser :type "Actor Object Reference"))
  (bind _returnvalue (`KismetMathLibrary.RandomFloatInRange` 0.0 1.0))
  (bind _bpc_health_component (`self.BPC_Health_Component`))
  (`/Game/My_Content/Player_Character/BPC_Health_Component.Decrease Health` _bpc_health_component Damage)
  (if (<= (`/Game/My_Content/Player_Character/BPC_Health_Component.Current_Health` _bpc_health_component) 0.0)
    (`AddComponent|NODE_AddParticleSystemComponent-0`)
    (`KismetArrayLibrary.Array_AddUnique` (`self.Ignore Actors`) self)
    (`GameplayStatics.ApplyRadialDamage` (`self.Damage`) (`SceneComponent.K2_GetComponentLocation` (`self.Mesh`)) 300.0 null (`self.Ignore Actors`) null null true)
    (`PrimitiveComponent.AddImpulse` (`self.Mesh`) (`KismetMathLibrary.MakeVector` (* _returnvalue 5000.0) (* _returnvalue 5000.0) 10000.0) "None" false)
    (`KismetSystemLibrary.Delay` 3.0)
    (`self.K2_DestroyActor`)))

(fn `UserConstructionScript`)