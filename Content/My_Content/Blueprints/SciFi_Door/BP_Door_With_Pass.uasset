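; Sci-fi door that requires a numpad password to open, with two panels that slide vertically apart.
; Interact, gated by Activated, shows a lazily created WB_Numpad holding the Password and a self reference, switching input to UI only.
; If already open, it instead calls OpenCloseDoor on PlayerRef and clears IsOpen.
; Open_Close_Door flip-flops a timeline forward and backward, lerping both panels between offsets computed at BeginPlay.
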(event `self.ReceiveBeginPlay`
  (bind _output_get (set `self.Start_Bottom_Door_Part_Loc` (`SceneComponent.RelativeLocation` (`self.Door_Bottom_Part`))))
  (set `self.End_Bottom_Door_Part_Loc` (`KismetMathLibrary.MakeVector` (.x _output_get) (.y _output_get) (- (.z _output_get) 300.0)))
  (bind _output_get_2 (set `self.Start_Upper_Door_Part_Loc` (`SceneComponent.RelativeLocation` (`self.Door_Upper_Part`))))
  (set `self.End_Upper_Door_Part_Loc` (`KismetMathLibrary.MakeVector` (.x _output_get_2) (.y _output_get_2) (- (.z _output_get_2) -350.0))))

(event `/Game/My_Content/Blueprints/SciFi_Door/BPI_Interactable.Interact`
  (params (PlayerRef :type "/Game/My_Content/Player_Character/BP_Player_Character Object Reference"))
  (bind _returnvalue (`GameplayStatics.GetPlayerController` 0))
  (if (`self.activated?`)
    (if (`self.is_Open?`)
      (`/Game/My_Content/Player_Character/BP_Player_Character.Open_Close_Door` PlayerRef null)
      (set `self.is_Open?` false)
      (else
        (`/Engine/EditorBlueprintResources/StandardMacros.IsValid` (`self.WB_Numpad`)
          (:`Is Valid`
            _)
          (:`Is Not Valid`
            (bind _returnvalue_2 (`|CreateWidget` "/Game/My_Content/Blueprints/SciFi_Door/WB_Numpad.WB_Numpad_C" (`GameplayStatics.GetPlayerController` 0) (`self.Password`) self))
            (set `self.WB_Numpad` _returnvalue_2)))
        (`UserWidget.AddToViewport` (`self.WB_Numpad`) 0)
        (set `PlayerController.bShowMouseCursor` true _returnvalue)
        (`WidgetBlueprintLibrary.SetInputMode_UIOnlyEx` _returnvalue (`self.WB_Numpad`) "LockAlways")))))

(event `Open_Close_Door`
  (if (`self.activated?`)
    (`/Engine/EditorBlueprintResources/StandardMacros.FlipFlop`
      (:`A`
        (bind (_direction _alpha) (`Timeline|Timeline_Alpa_Loc` :!label _label)
          (:`Update`
            (`SceneComponent.K2_SetRelativeLocation` (`self.Door_Bottom_Part`) (`KismetMathLibrary.VLerp` (`self.Start_Bottom_Door_Part_Loc`) (`self.End_Bottom_Door_Part_Loc`) _alpha) false false)
            (`SceneComponent.K2_SetRelativeLocation` (`self.Door_Upper_Part`) (`KismetMathLibrary.VLerp` (`self.Start_Upper_Door_Part_Loc`) (`self.End_Upper_Door_Part_Loc`) _alpha) false false))))
      (:`B`
        (goto _label :!via `Reverse`)))))

(fn `UserConstructionScript`)