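; Base weapon Blueprint that handles pickup into a character's inventory and gates firing and reloading.
; PickUp registers the weapon and owner, equips the first inventory entry and disables physics and collision; if already in inventory, it only clears that flag.
; Fire and reload checks test magazine count and equipped state, emitting AI noise from the owner when they pass.
; Fire, Reload and EquipUnequip are empty here.
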(event `/Game/My_Content/Weapons/BPI_Pickup.PickUp`
  (params (Character_Ref :type "/Game/My_Content/Player_Character/BP_Player_Character Object Reference"))
  (bind _mesh (`self.Mesh`))
  (bind _inventory_weapons (`/Game/My_Content/Player_Character/BP_Player_Character.Inventory_Weapons` Character_Ref))
  (bind _gun_owner (`self.Gun_Owner`))
  (if (`self.In_Character_Inventory?`)
    (set `self.In_Character_Inventory?` false)
    (else
      (`KismetArrayLibrary.Array_AddUnique` _inventory_weapons self)
      (set `self.Gun_Owner` Character_Ref)
      (set `self.In_Character_Inventory?` true)
      (if (> (`KismetArrayLibrary.Array_Length` _inventory_weapons) 0)
        (set `/Game/My_Content/Player_Character/BP_Player_Character.Equiped_Weapon` (`|GetArrayItem` (`/Game/My_Content/Player_Character/BP_Player_Character.Inventory_Weapons` _gun_owner)) _gun_owner)
        (if (`self.In_Character_Inventory?`)
          (`PrimitiveComponent.SetSimulatePhysics` _mesh false)
          (`PrimitiveComponent.SetCollisionObjectType` _mesh "ECC_WorldStatic")
          (`PrimitiveComponent.SetCollisionEnabled` _mesh "NoCollision")
          (`PrimitiveComponent.SetCollisionEnabled` (`self.Capsule`) "NoCollision"))))))

(fn `Check_Can_Fire`
  (returns (`Can_Fire?` :type Boolean))
  (if (and (> (`self.Magazine_Capacity`) 0) (`self.Is_Equipped?`))
    ;[1 1 1] Make Noise For AI
    (`self.MakeNoise` (`self.Gun_Owner`) 1.0 null (`SceneComponent.K2_GetComponentLocation` (`self.Mesh`)) 0.0 "None")
    (return true)
    (else
      (return false))))

(fn `Check_Can_Reload`
  (returns (`Can_Reload?` :type Boolean))
  (if (and (< (`self.Magazine_Capacity`) (`self.Max_Magazine_Capacity`)) (`self.Is_Equipped?`))
    ;[1 1 1] Make Noise For AI
    (`self.MakeNoise` (`self.Gun_Owner`) 1.0 null (`SceneComponent.K2_GetComponentLocation` (`self.Mesh`)) 0.0 "None")
    (return true)
    (else
      (return false))))

(fn `Equip Unequip`)

(fn `Fire`)

(fn `Reload`)

(fn `UserConstructionScript`)