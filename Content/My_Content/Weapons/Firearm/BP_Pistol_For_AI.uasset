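; AI pistol weapon, a child Blueprint that attaches to its owner's right hand socket on pickup.
; Fire plays the weapon animation, spends a round, line traces from the muzzle, applies damage and prints the hit actor's name.
; A helper ejects a physics-simulated bullet actor and places a bullet-hole decal at the hit.
; Reload plays a montage on the owner behind a DoOnce, blocking fire until completion refills the magazine.
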(event `self.ReceiveBeginPlay`
  (`parent.ReceiveBeginPlay`))

(event `self.ReceiveTick`
  (params (DeltaSeconds :type "Float (single-precision)"))
  (`parent.ReceiveTick` DeltaSeconds))

(event `self.PickUp`
  (params (Character_Ref :type "/Game/My_Content/AI/BP_AI_Char Object Reference"))
  (`parent.PickUp` Character_Ref)
  (`SceneComponent.K2_AttachToComponent` (`self.Mesh`) (`Character.Mesh` (`self.Gun_Owner`)) "Right_hand" "SnapToTarget" "SnapToTarget" "KeepWorld" true))

(event `self.Fire`
  (bind _mesh (`self.Mesh`))
  (bind _mesh_2 (`self.Mesh`))
  (bind _returnvalue (`SceneComponent.GetSocketLocation` _mesh "MuzzleFlash"))
  (bind _returnvalue_2 (`SceneComponent.GetSocketRotation` _mesh_2 "AmmoEject"))
  (bind _can_fire_ (`self.Check_Can_Fire`))
  (if _can_fire_
    (`SkeletalMeshComponent.PlayAnimation` (`self.Mesh`) "/Game/MilitaryWeapDark/Weapons/Anims/Fire_Pistol_W.Fire_Pistol_W" false)
    ;[1 1 1] Minusing Bullet
    (if (> (`self.Magazine_Capacity`) 0)
      (set `self.Magazine_Capacity` (- (`self.Magazine_Capacity`) 1))
      (bind _outhit (`KismetSystemLibrary.LineTraceSingle` _returnvalue (+ _returnvalue (* (`SceneComponent.GetSocketRotation` _mesh "MuzzleFlash") 1000000.0)) "TraceTypeQuery2"))
      (bind _returnvalue_3 (`|SpawnActorFromClass` "/Game/My_Content/Weapons/Firearm/BP_Pistol_Bullet.BP_Pistol_Bullet_C" (`SceneComponent.GetSocketTransform` _mesh_2 "AmmoEject" "RTS_World") "Undefined" "MultiplyWithRoot" null null))
      (bind _mesh_3 (`/Game/My_Content/Weapons/Firearm/BP_Pistol_Bullet.Mesh` _returnvalue_3))
      (`PrimitiveComponent.SetSimulatePhysics` _mesh_3 true)
      (`PrimitiveComponent.AddImpulse` _mesh_3 (* (+ (`KismetMathLibrary.GetUpVector` _returnvalue_2) (`KismetMathLibrary.GetRightVector` _returnvalue_2)) (`KismetMathLibrary.RandomIntegerInRange` 5 7)) "None" false)
      (`GameplayStatics.SpawnDecalAtLocation` "/Game/My_Content/Weapons/Decals/M_Bullet_Hole.M_Bullet_Hole" (`KismetMathLibrary.Conv_DoubleToVector` (`KismetMathLibrary.RandomFloatInRange` 5.0 7.0)) (`.Location` (`GameplayStatics.BreakHitResult` _outhit)) (`KismetMathLibrary.Conv_VectorToRotator` (`.ImpactNormal` (`GameplayStatics.BreakHitResult` _outhit))) 30.0)
      (`KismetSystemLibrary.PrintString` (`KismetSystemLibrary.GetDisplayName` (`.HitActor` (`GameplayStatics.BreakHitResult` _outhit))))
      (`GameplayStatics.ApplyDamage` (`.HitActor` (`GameplayStatics.BreakHitResult` _outhit)) (`self.Damage`) null self))))

(event `self.Reload`
  (bind _gun_owner (`self.Gun_Owner`))
  (bind _can_reload_ (`self.Check_Can_Reload`))
  (if _can_reload_
    (`/Engine/EditorBlueprintResources/StandardMacros.DoOnce` false :!label _label
      (:`Completed`
        (`|PlayMontage` (`Character.Mesh` (`self.Gun_Owner`)) "/Game/My_Content/Animations/Player_Character/Sequences/Weapon_Actions/AM_Pistol_Reload.AM_Pistol_Reload"
          (:`then`
            (set `/Game/My_Content/AI/BP_AI_Char.can_Fire?` false (`self.Gun_Owner`)))
          (:`OnCompleted`
            (set `self.Magazine_Capacity` (`self.Max_Magazine_Capacity`))
            (set `/Game/My_Content/AI/BP_AI_Char.can_Fire?` true _gun_owner)
            (set `/Game/My_Content/AI/BP_AI_Char.is_Reloading?` false _gun_owner)
            (goto _label :!via `Reset`)))))))

(fn `UserConstructionScript`
  (`parent.UserConstructionScript`))