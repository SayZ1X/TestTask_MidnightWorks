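; Pistol weapon Blueprint, a child of a gun base, that handles holstering, hitscan firing and reloading for its owner.
; Pickup snaps it to the holster socket, and equip montage notifies move it between holster and right hand.
; Firing spends a round, traces from the muzzle, applies damage, ejects a physics bullet actor, places a decal and makes AI noise.
; Reload is DoOnce-guarded, refilling the magazine when its montage completes.
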(event `self.ReceiveBeginPlay`
  (`parent.ReceiveBeginPlay`))

(event `self.ReceiveTick`
  (params (DeltaSeconds :type "Float (single-precision)"))
  (`parent.ReceiveTick` DeltaSeconds))

(event `/Game/My_Content/Weapons/BPI_Pickup.PickUp`
  (params (Character_Ref :type "/Game/My_Content/Player_Character/BP_Player_Character Object Reference"))
  (`parent.PickUp` Character_Ref)
  (`SceneComponent.K2_AttachToComponent` (`self.Mesh`) (`Character.Mesh` (`self.Gun_Owner`)) "Pistol_holster" "SnapToTarget" "SnapToTarget" "KeepWorld" true))

(event `self.Equip Unequip`
  (bind _mesh (`Character.Mesh` (`self.Gun_Owner`)))
  (if (`self.Is_Equipped?`)
    (set `self.Is_Equipped?` false)
    (set `self.Socket_Name` "Pistol_holster")
    (`|PlayMontage` _mesh "/Game/My_Content/Animations/Player_Character/Sequences/Weapon_Actions/AM_Equip_Pistol_Reverse.AM_Equip_Pistol_Reverse"
      (:`OnNotifyBegin`
        _))
    (else
      (set `self.Is_Equipped?` true)
      (set `self.Socket_Name` "Right_hand")
      (`|PlayMontage` _mesh "/Game/My_Content/Animations/Player_Character/Sequences/Weapon_Actions/AM_Equip_Pistol.AM_Equip_Pistol"
        (:`OnNotifyBegin`
          _))))
  (`SceneComponent.K2_AttachToComponent` (`self.Mesh`) (`Character.Mesh` (`self.Gun_Owner`)) (`self.Socket_Name`) "SnapToTarget" "SnapToTarget" "KeepWorld" true))

(event `self.Fire`
  (bind _mesh (`self.Mesh`))
  (bind _mesh_2 (`self.Mesh`))
  (bind _returnvalue (`SceneComponent.GetSocketLocation` _mesh "MuzzleFlash"))
  (bind _returnvalue_2 (`SceneComponent.GetSocketRotation` _mesh_2 "AmmoEject"))
  (bind _can_fire_ (`self.Check_Can_Fire`))
  (if _can_fire_
    (`SkeletalMeshComponent.PlayAnimation` (`self.Mesh`) "/Game/MilitaryWeapDark/Weapons/Anims/Fire_Pistol_W.Fire_Pistol_W" false)
    ;[1 1 1] Minusing Bullet
    (if (> (`self.Magazine_Capacity`) 0)
      (set `self.Magazine_Capacity` (- (`self.Magazine_Capacity`) 1))
      (bind _outhit (`KismetSystemLibrary.LineTraceSingle` _returnvalue (+ _returnvalue (* (`SceneComponent.GetSocketRotation` _mesh "MuzzleFlash") 1000000.0)) "TraceTypeQuery2"))
      (bind _returnvalue_3 (`|SpawnActorFromClass` "/Game/My_Content/Weapons/Firearm/BP_Pistol_Bullet.BP_Pistol_Bullet_C" (`SceneComponent.GetSocketTransform` _mesh_2 "AmmoEject" "RTS_World") "Undefined" "MultiplyWithRoot" null null))
      (bind _mesh_3 (`/Game/My_Content/Weapons/Firearm/BP_Pistol_Bullet.Mesh` _returnvalue_3))
      (`PrimitiveComponent.SetSimulatePhysics` _mesh_3 true)
      (`PrimitiveComponent.AddImpulse` _mesh_3 (* (+ (`KismetMathLibrary.GetUpVector` _returnvalue_2) (`KismetMathLibrary.GetRightVector` _returnvalue_2)) (`KismetMathLibrary.RandomIntegerInRange` 5 7)) "None" false)
      (`GameplayStatics.SpawnDecalAtLocation` "/Game/My_Content/Weapons/Decals/M_Bullet_Hole.M_Bullet_Hole" (`KismetMathLibrary.Conv_DoubleToVector` (`KismetMathLibrary.RandomFloatInRange` 5.0 7.0)) (`.Location` (`GameplayStatics.BreakHitResult` _outhit)) (`KismetMathLibrary.Conv_VectorToRotator` (`.ImpactNormal` (`GameplayStatics.BreakHitResult` _outhit))) 30.0)
      (`GameplayStatics.ApplyDamage` (`.HitActor` (`GameplayStatics.BreakHitResult` _outhit)) (`self.Damage`) null self)
      ;[1 1 1] Make Noise For AI
      (`self.MakeNoise` (`self.Gun_Owner`) 1.0 null (`SceneComponent.K2_GetComponentLocation` (`self.Mesh`)) 0.0 "None"))))

(event `self.Reload`
  (bind _gun_owner (`self.Gun_Owner`))
  (bind _can_reload_ (`self.Check_Can_Reload`))
  (if _can_reload_
    (`/Engine/EditorBlueprintResources/StandardMacros.DoOnce` false :!label _label
      (:`Completed`
        (`|PlayMontage` (`Character.Mesh` (`self.Gun_Owner`)) "/Game/My_Content/Animations/Player_Character/Sequences/Weapon_Actions/AM_Pistol_Reload.AM_Pistol_Reload"
          (:`then`
            (set `/Game/My_Content/Player_Character/BP_Player_Character.can_Fire?` false _gun_owner))
          (:`OnCompleted`
            (set `self.Magazine_Capacity` (`self.Max_Magazine_Capacity`))
            (set `/Game/My_Content/Player_Character/BP_Player_Character.can_Fire?` true _gun_owner)
            (set `/Game/My_Content/Player_Character/BP_Player_Character.is_Reloading?` false (`self.Gun_Owner`))
            (goto _label :!via `Reset`)))))))

(fn `UserConstructionScript`
  (`parent.UserConstructionScript`))