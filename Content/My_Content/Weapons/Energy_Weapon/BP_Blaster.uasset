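; BP_Blaster is an energy pistol weapon, derived from a parent gun class, that attaches to the character's holster on pickup.
; Equip toggling plays forward or reverse montages, moving the mesh between hand and holster sockets on a montage notify.
; Firing spawns an actor at the muzzle with sound and a brief Niagara flash, decrementing the magazine.
; Reloading uses a DoOnce-guarded montage, blocking fire until completion refills the magazine.
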(event `self.ReceiveTick`
  (params (DeltaSeconds :type "Float (single-precision)"))
  (`parent.ReceiveTick` DeltaSeconds))

(event `/Game/My_Content/Weapons/BPI_Pickup.PickUp`
  (params (Character_Ref :type "/Game/My_Content/Player_Character/BP_Player_Character Object Reference"))
  (`parent.PickUp` Character_Ref)
  (`SceneComponent.K2_AttachToComponent` (`self.Mesh`) (`Character.Mesh` (`self.Gun_Owner`)) "Blaster_holster" "SnapToTarget" "SnapToTarget" "KeepWorld" true))

(event `self.Equip Unequip`
  (bind _mesh (`Character.Mesh` (`self.Gun_Owner`)))
  (if (`self.Is_Equipped?`)
    (set `self.Is_Equipped?` false)
    (set `self.Socket Name` "Blaster_holster")
    (`|PlayMontage` _mesh "/Game/My_Content/Animations/Player_Character/Sequences/Weapon_Actions/AM_Equip_Pistol_Reverse.AM_Equip_Pistol_Reverse"
      (:`OnNotifyBegin`
        _))
    (else
      (set `self.Is_Equipped?` true)
      (set `self.Socket Name` "Right_hand_blaster")
      (`|PlayMontage` _mesh "/Game/My_Content/Animations/Player_Character/Sequences/Weapon_Actions/AM_Equip_Pistol.AM_Equip_Pistol"
        (:`OnNotifyBegin`
          _))))
  (`SceneComponent.K2_AttachToComponent` (`self.Mesh`) (`Character.Mesh` (`self.Gun_Owner`)) (`self.Socket Name`) "SnapToTarget" "SnapToTarget" "SnapToTarget" true))

(event `self.Fire`
  (bind _mesh (`self.Mesh`))
  (bind _mesh_2 (`self.Mesh`))
  (bind _can_fire_ (`self.Check_Can_Fire`))
  (if _can_fire_
    (`GameplayStatics.PlaySoundAtLocation` "/Game/My_Content/Sounds/MS_Energy_Projectile_Shoot.MS_Energy_Projectile_Shoot" (`SceneComponent.GetSocketLocation` _mesh_2 "Muzzle") (struct) 1.0 1.0 0.0 null null null null)
    (`|SpawnActorFromClass` "/Game/My_Content/Weapons/Energy_Weapon/BP_Energy_Projectile.BP_Energy_Projectile_C" (`SceneComponent.GetSocketTransform` _mesh_2 "Muzzle" "RTS_World") "AlwaysSpawn" "MultiplyWithRoot" (`self.Gun_Owner`) null)
    ;[1 1 1] Minusing Bullet
    (if (> (`self.Magazine_Capacity`) 0)
      (set `self.Magazine_Capacity` (- (`self.Magazine_Capacity`) 1))
      (bind _returnvalue (`NiagaraFunctionLibrary.SpawnSystemAtLocation` "/Game/RocketThrusterExhaustFX/FX/NS_RocketExhaust_Violet.NS_RocketExhaust_Violet" (`SceneComponent.GetSocketLocation` _mesh "Muzzle") (`SceneComponent.GetSocketRotation` _mesh "Muzzle") (0.3 0.3 1.0)))
      (`KismetSystemLibrary.Delay` 0.2)
      (`ActorComponent.K2_DestroyComponent` _returnvalue))))

(event `self.Reload`
  (bind _gun_owner (`self.Gun_Owner`))
  (bind _can_reload_ (`self.Check_Can_Reload`))
  (if _can_reload_
    (`/Engine/EditorBlueprintResources/StandardMacros.DoOnce` false :!label _label
      (:`Completed`
        (`|PlayMontage` (`Character.Mesh` (`self.Gun_Owner`)) "/Game/My_Content/Animations/Player_Character/Sequences/Weapon_Actions/AM_Pistol_Reload.AM_Pistol_Reload"
          (:`then`
            (set `/Game/My_Content/Player_Character/BP_Player_Character.can_Fire?` false _gun_owner))
          (:`OnCompleted`
            (set `self.Magazine_Capacity` (`self.Max_Magazine_Capacity`))
            (set `/Game/My_Content/Player_Character/BP_Player_Character.can_Fire?` true _gun_owner)
            (set `/Game/My_Content/Player_Character/BP_Player_Character.is_Reloading?` false (`self.Gun_Owner`))
            (goto _label :!via `Reset`)))))))

(fn `UserConstructionScript`
  (`parent.UserConstructionScript`))