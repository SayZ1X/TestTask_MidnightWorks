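; Energy weapon projectile that explodes on impact and deals radial damage.
; On spawn, its collision sphere ignores the owning actor while moving.
; When projectile movement stops, it plays a hit sound, leaves a randomly sized temporary bullet-hole decal aligned to the surface, spawns an explosion and applies area damage.
; It then has the owner report noise at the impact point for AI and destroys itself.
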(event `self.ReceiveBeginPlay`
  (`PrimitiveComponent.IgnoreActorWhenMoving` (`self.Sphere`) (`self.GetOwner`) true))

(event `self.ProjectileMovement.OnProjectileStop`
  (params (ImpactResult :type "HitResult Structure (by ref)"))
  (`GameplayStatics.PlaySoundAtLocation` "/Game/My_Content/Sounds/MS_Energy_Projectile_Hit.MS_Energy_Projectile_Hit" ImpactResult_Location (struct) 1.0 1.0 0.0 null null null null)
  (`GameplayStatics.SpawnDecalAtLocation` "/Game/My_Content/Weapons/Decals/M_Bullet_Hole.M_Bullet_Hole" (`KismetMathLibrary.Conv_IntToVector` (`KismetMathLibrary.RandomIntegerInRange` 13 18)) ImpactResult_Location (`KismetMathLibrary.MakeRotFromX` ImpactResult_Normal) 30.0)
  (`GameplayStatics.SpawnEmitterAtLocation` "/Game/StarterContent/Particles/P_Explosion.P_Explosion" ImpactResult_Location (struct) (3.0 3.0 3.0))
  (`GameplayStatics.ApplyRadialDamage` :`BaseDamage` (`self.Damage`) :`Origin` ImpactResult_Location :`DamageRadius` 250.0 :`DamageCauser` null :`InstigatedByController` null)
  ;[1 1 1] Make Noise For AI
  (`self.MakeNoise` (`self.GetOwner`) 1.0 null ImpactResult_Location 0.0 "None")
  (`self.K2_DestroyActor`))

(fn `UserConstructionScript`)